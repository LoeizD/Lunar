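; Handheld build device that places and sizes BP_LunarCube blocks in BuildMode.
; On the server, successive fire presses spawn a cube at the trace hit, lock its XY footprint, then lock height and call SetGoodMat.
; Server Tick drives the cube's clamped Scale from the offset between its origin and the ray's fixed-distance endpoint.
; On remote instances, Tick line-traces to position and show the Target marker.
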(event `self.ReceiveTick`
  (params (DeltaSeconds :type "Float (single-precision)"))
  (bind _mesh (`self.Mesh`))
  (bind (_blocorigin_x _blocorigin_y _blocorigin_z) (`KismetMathLibrary.BreakVector` (`self.BlocOrigin`)))
  (bind _target (`self.Target`))
  (bind _mesh_2 (`self.Mesh`))
  (bind _returnvalue (`SceneComponent.K2_GetComponentLocation` _mesh_2))
  (bind (_returnvalue_x _returnvalue_y) (`KismetMathLibrary.BreakVector` (`self.GetActorScale3D` (`self.Bloc`))))
  (bind (_returnvalue_x_2 _returnvalue_y_2 _returnvalue_z) (`KismetMathLibrary.BreakVector` (+ (`SceneComponent.K2_GetComponentLocation` _mesh) (* (`SceneComponent.GetForwardVector` _mesh) (`self.RayDist`)))))
  (`|ExecutionSequence`
    (:`then_0`
      (`/Engine/EditorBlueprintResources/ActorMacros.Switch Has Authority`
        (:`Authority`
          (if (`self.BuildMode?`)
            (if (`self.BlocXY`)
              (set `/Game/RestrictedAssets/Tutorials/Lunar/BP_LunarCube.Scale` (`KismetMathLibrary.MakeVector` (`KismetMathLibrary.FClamp` (/ (- _blocorigin_x _returnvalue_x_2) 100.0) -15.0 15.0) (`KismetMathLibrary.FClamp` (/ (- _returnvalue_y_2 _blocorigin_y) -100.0) -15.0 15.0)) (`self.Bloc`))
              (elif (`self.BlocZ`)
                (set `/Game/RestrictedAssets/Tutorials/Lunar/BP_LunarCube.Scale` (`KismetMathLibrary.MakeVector` _returnvalue_x _returnvalue_y (`KismetMathLibrary.FClamp` (/ (- _returnvalue_z _blocorigin_z) 75.0) -10.0 10.0)) (`self.Bloc`))))))))
    (:`then_1`
      (`/Engine/EditorBlueprintResources/ActorMacros.Switch Has Authority`
        (:`Remote`
          (bind (_outhit _returnvalue_2) (`KismetSystemLibrary.LineTraceSingle` _returnvalue (+ _returnvalue (* (`SceneComponent.GetForwardVector` _mesh_2) (`self.RayDist`))) "TraceTypeQuery1"))
          (`SceneComponent.SetVisibility` _target _returnvalue_2 false)
          (if _returnvalue_2
            (`SceneComponent.K2_SetWorldLocation` _target (`.Location` (`GameplayStatics.BreakHitResult` _outhit)) false false)))))))

(event `self.OnStartedFiring`
  (bind _mesh (`self.Mesh`))
  (bind _returnvalue (`SceneComponent.K2_GetComponentLocation` _mesh))
  (`/Engine/EditorBlueprintResources/ActorMacros.Switch Has Authority`
    (:`Authority`
      (if (`self.End?`) :!label _label
        _
        (elif (`self.BuildMode?`)
          (if (`self.BlocBegin`)
            (bind (_outhit _returnvalue_2) (`KismetSystemLibrary.LineTraceSingle` :`Start` _returnvalue :`End` (+ _returnvalue (* (`SceneComponent.GetForwardVector` _mesh) (`self.RayDist`))) :`TraceChannel` "TraceTypeQuery1" :`DrawDebugType` "ForOneFrame"))
            (if _returnvalue_2
              (bind _output_get (set `self.BlocOrigin` (`.Location` (`GameplayStatics.BreakHitResult` _outhit))))
              (bind _returnvalue_3 (`|SpawnActorFromClass` "/Game/RestrictedAssets/Tutorials/Lunar/BP_LunarCube.BP_LunarCube_C" (`KismetMathLibrary.MakeTransform` _output_get (struct) (0.1 0.1 0.1)) "Undefined" "OverrideRootScale"))
              (set `self.Bloc` _returnvalue_3)
              (set `self.BlocBegin` false)
              (set `self.BlocXY` true)
              (else
                (`KismetSystemLibrary.PrintString` "NoCollision")))
            (elif (`self.BlocXY`)
              (set `self.BlocXY` false)
              (set `self.BlocZ` true)
              (elif (`self.BlocZ`)
                (set `self.BlocBegin` true)
                (set `self.BlocZ` false)
                (`/Engine/EditorBlueprintResources/ActorMacros.Switch Has Authority`
                  (:`Authority`
                    (`/Game/RestrictedAssets/Tutorials/Lunar/BP_LunarCube.SetGoodMat` (`self.Bloc`))))))))))))

(event `LunarBuild`
  (goto _label))

(fn `FireShotOverride`
  (returns (ReturnValue :type Boolean))
  (return false))

(fn `UserConstructionScript`)