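; Lunar device that lets a player place and size BP_LunarCube blocks in build mode.
; Each E press advances a state machine: spawn at the camera trace hit, lock XY size, then lock height and call SetGoodMat.
; Tick scales the block from camera aim and moves a target marker on remote instances.
; Spawning runs with authority; ClientRequest maps the PlayerState to a player index for camera lookup.
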(event `self.ReceiveTick`
  (params (DeltaSeconds :type "Float (single-precision)"))
  (bind (_blocorigin_x _blocorigin_y _blocorigin_z) (`KismetMathLibrary.BreakVector` (`self.BlocOrigin`)))
  (bind _target (`self.Target`))
  (bind _mesh (`self.Mesh`))
  (bind _returnvalue (`GameplayStatics.GetPlayerCameraManager` (`self.PlayerIndex`)))
  (bind _returnvalue_2 (`SceneComponent.K2_GetComponentLocation` _mesh))
  (bind (_returnvalue_x _returnvalue_y) (`KismetMathLibrary.BreakVector` (`self.GetActorScale3D` (`self.Bloc`))))
  (bind (_returnvalue_x_2 _returnvalue_y_2 _returnvalue_z) (`KismetMathLibrary.BreakVector` (+ (`PlayerCameraManager.GetCameraLocation` _returnvalue) (* (`KismetMathLibrary.GetForwardVector` (`PlayerCameraManager.GetCameraRotation` _returnvalue)) (`self.RayDist`)))))
  (`|ExecutionSequence`
    (:`then_0`
      (`/Engine/EditorBlueprintResources/ActorMacros.Switch Has Authority`
        (:`Authority`
          _)
        (:`Remote`
          _))
      (if (`self.BuildMode?`)
        (if (`self.BlocXY`)
          (set `/Game/RestrictedAssets/Tutorials/Lunar/BP_LunarCube.Scale` (`KismetMathLibrary.MakeVector` (`KismetMathLibrary.FClamp` (/ (- _blocorigin_x _returnvalue_x_2) 100.0) -15.0 15.0) (`KismetMathLibrary.FClamp` (/ (- _returnvalue_y_2 _blocorigin_y) -100.0) -15.0 15.0)) (`self.Bloc`))
          (elif (`self.BlocZ`)
            (set `/Game/RestrictedAssets/Tutorials/Lunar/BP_LunarCube.Scale` (`KismetMathLibrary.MakeVector` _returnvalue_x _returnvalue_y (`KismetMathLibrary.FClamp` (/ (- _returnvalue_z _blocorigin_z) 75.0) -10.0 10.0)) (`self.Bloc`))))))
    (:`then_1`
      (`/Engine/EditorBlueprintResources/ActorMacros.Switch Has Authority`
        (:`Remote`
          (bind (_outhit _returnvalue_3) (`KismetSystemLibrary.LineTraceSingle` _returnvalue_2 (+ _returnvalue_2 (* (`SceneComponent.GetForwardVector` _mesh) (`self.RayDist`))) "TraceTypeQuery1"))
          (`SceneComponent.SetVisibility` _target _returnvalue_3 false)
          (if _returnvalue_3
            (`SceneComponent.K2_SetWorldLocation` _target (`.Location` (`GameplayStatics.BreakHitResult` _outhit)) false false)))))
    (:`then_2`
      (if (`PlayerController.WasInputKeyJustPressed` (`GameplayStatics.GetPlayerController` 0) "E")
        (`self.CustomKey`)))))

(event `CustomKey`
  (bind _returnvalue (`GameplayStatics.GetPlayerCameraManager` (`self.PlayerIndex`)))
  (bind _returnvalue_2 (`PlayerCameraManager.GetCameraLocation` _returnvalue))
  (`/Engine/EditorBlueprintResources/ActorMacros.Switch Has Authority`
    (:`Authority`
      (if (== (`self.GetOwner`) (`GameplayStatics.GetPlayerPawn` 0))
        (set `self.PlayerIndex` 0)
        (if (`self.End?`) :!label _label
          _
          (elif (`self.BuildMode?`)
            (if (`self.BlocBegin`)
              (bind (_outhit _returnvalue_3) (`KismetSystemLibrary.LineTraceSingle` :`Start` _returnvalue_2 :`End` (+ _returnvalue_2 (* (`KismetMathLibrary.GetForwardVector` (`PlayerCameraManager.GetCameraRotation` _returnvalue)) (`self.RayDist`))) :`TraceChannel` "TraceTypeQuery1" :`DrawDebugType` "ForOneFrame"))
              (if _returnvalue_3
                (bind _output_get (set `self.BlocOrigin` (`.Location` (`GameplayStatics.BreakHitResult` _outhit))))
                (`KismetSystemLibrary.PrintString` "SpawnLCube")
                (bind _returnvalue_4 (`|SpawnActorFromClass` "/Game/RestrictedAssets/Tutorials/Lunar/BP_LunarCube.BP_LunarCube_C" (`KismetMathLibrary.MakeTransform` _output_get (struct) (0.1 0.1 0.1)) "Undefined" "OverrideRootScale"))
                (set `self.Bloc` _returnvalue_4)
                (set `self.BlocBegin` false)
                (set `self.BlocXY` true)
                (else
                  (`KismetSystemLibrary.PrintString` "NoCollision")))
              (elif (`self.BlocXY`)
                (set `self.BlocXY` false)
                (set `self.BlocZ` true)
                (elif (`self.BlocZ`)
                  (set `self.BlocBegin` true)
                  (set `self.BlocZ` false)
                  (`/Engine/EditorBlueprintResources/ActorMacros.Switch Has Authority`
                    (:`Authority`
                      _)
                    (:`Remote`
                      _))
                  (`/Game/RestrictedAssets/Tutorials/Lunar/BP_LunarCube.SetGoodMat` (`self.Bloc`)))))))))
    (:`Remote`
      (`self.ClientRequest` (`Pawn.PlayerState` (`GameplayStatics.GetPlayerPawn` 0))))))

(event `ClientRequest`
  (params (PlayerState :type "PlayerState Object Reference"))
  (`KismetSystemLibrary.PrintString` "cliReq")
  (`/Engine/EditorBlueprintResources/ActorMacros.Switch Has Authority`
    (:`Authority`
      (for (_array_element _array_index) (`GameStateBase.PlayerArray` (`GameplayStatics.GetGameState`))
        (if (== _array_element PlayerState)
          (set `self.PlayerIndex` _array_index)))
      (goto _label))))

(fn `FireShotOverride`
  (returns (ReturnValue :type Boolean))
  (return false))

(fn `UserConstructionScript`)