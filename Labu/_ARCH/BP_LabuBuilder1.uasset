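; Player-owned building tool that places wall, floor or slope tiles from a hologram preview, with key selection and a cooldown UI.
; Tick polls keys; holding build spawns a first tile, then camera and velocity-offset downward traces chain tiles onto "holo"-tagged components.
; When its owner becomes invalid, it clears holos and spawns a health pack.
; An older stretch-to-size cube builder (B1) remains, its triggers disconnected.
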(event `ClientRequestTick`
  (params (PlayerState :type "PlayerState Object Reference"))
  (bind _build1_impactpoint (`self.Build1_ImpactPoint`))
  (bind _build1_holocube (`self.Build1_HoloCube`))
  (bind _returnvalue (`GameplayStatics.GetPlayerCameraManager` (`self.PlayerIndex`)))
  (bind _buildtarget (`/Game/RestrictedAssets/Tutorials/Lunar/Labu/_ARCH/BP_BuildWall1.BuildTarget` (`self.Build1_CurrentBuildWall`)))
  (bind (_returnvalue_x _returnvalue_y) (`KismetMathLibrary.BreakVector` (`PlayerCameraManager.GetCameraLocation` (`GameplayStatics.GetPlayerCameraManager` (`self.PlayerIndex`)))))
  (bind _returnvalue_2 (`PlayerCameraManager.GetCameraLocation` _returnvalue))
  (bind (_relativelocation_x _relativelocation_y _relativelocation_z) (`KismetMathLibrary.BreakVector` (`SceneComponent.RelativeLocation` _buildtarget)))
  (bind _returnvalue_3 (`KismetMathLibrary.MakeRotFromZX` (`self.Build1_Normal`) (- (`KismetMathLibrary.MakeVector` _returnvalue_x _returnvalue_y (.z _build1_impactpoint)) _build1_impactpoint)))
  ;[1 0 0] B1 old
  (`/Engine/EditorBlueprintResources/ActorMacros.Switch Has Authority`
    (:`Authority`
      (for (_array_element _array_index) (`GameStateBase.PlayerArray` (`GameplayStatics.GetGameState`))
        (if (== _array_element PlayerState)
          (set `self.PlayerIndex` _array_index)))
      (if (`self.Build1_IsBuilding`)
        (bind _outhit (`KismetSystemLibrary.LineTraceSingle` :`Start` _returnvalue_2 :`End` (+ _returnvalue_2 (* (`self.GetActorForwardVector` _returnvalue) 1000.0)) :`TraceChannel` "TraceTypeQuery1" :`TraceColor` (struct :`G` 1.0 :`B` 1.0 :`A` 1.0) :`TraceHitColor` (struct :`R` 1.0 :`B` 0.930164 :`A` 1.0)))
        (`SceneComponent.K2_SetWorldLocation` _buildtarget (`.ImpactPoint` (`GameplayStatics.BreakHitResult` _outhit)) false false)
        (bind _output_get (set `self.CurrentScaleZ` (`KismetMathLibrary.FClamp` (* (select `bool` (> _relativelocation_z 0.1) :`false` 0.1 :`true` _relativelocation_z) 0.01) 0.1 10.0)))
        (bind _output_get_2 (set `self.CurrentScaleY` (`KismetMathLibrary.FClamp` (* (`KismetMathLibrary.Abs` _relativelocation_y) 0.02) 0.1 10.0)))
        ;;[1 1 1] useless?
        (set `self.CurrentScaleX` (`KismetMathLibrary.FClamp` (* (`KismetMathLibrary.Abs` _relativelocation_x) 0.02) 0.1 10.0))
        (set `/Game/RestrictedAssets/Tutorials/Lunar/Labu/_ARCH/BP_LunarCube_EditLabuBuild1.Scale` (`KismetMathLibrary.MakeVector` _output_get_2 _output_get_2 _output_get) _build1_holocube)
        (set `/Game/RestrictedAssets/Tutorials/Lunar/Labu/_ARCH/BP_LunarCube_EditLabuBuild1.Rotation` _returnvalue_3 _build1_holocube)
        (set `/Game/RestrictedAssets/Tutorials/Lunar/Labu/_ARCH/BP_BuildWall1.Rotation` _returnvalue_3 (`self.Build1_CurrentBuildWall`))))))

(event `self.ReceiveBeginPlay`
  ;[0.003576 1 0] BEGIN PLAY
  (`KismetSystemLibrary.Delay` 0.1)
  (if (== (`self.GetOwner`) (`GameplayStatics.GetPlayerPawn` 0))
    (`self.GetOrCreateUI`)
    (bind _returnvalue (`|SpawnActorFromClass` "/Game/RestrictedAssets/Tutorials/Lunar/Labu/BP_B3_HoloShapes.BP_B3_HoloShapes_C" (`KismetMathLibrary.MakeTransform` (0.0 0.0 0.0) (struct) (1.0 1.0 1.0)) "Undefined" "OverrideRootScale"))
    (set `self.REF_HoloShape` _returnvalue)
    (set `self.SM_HoloWall_REF` (`/Game/RestrictedAssets/Tutorials/Lunar/Labu/BP_B3_HoloShapes.SM_HoloWall` _returnvalue))
    (set `self.SM_HoloFloor_REF` (`/Game/RestrictedAssets/Tutorials/Lunar/Labu/BP_B3_HoloShapes.SM_HoloFloor` _returnvalue))
    (set `self.SM_HoloSlope_REF` (`/Game/RestrictedAssets/Tutorials/Lunar/Labu/BP_B3_HoloShapes.SM_HoloSlope` _returnvalue))
    (`self.B3KeyVPress`)))

(event `self.ReceiveTick`
  (params (DeltaSeconds :type "Float (single-precision)"))
  (bind _returnvalue (`self.GetOwner`))
  ;[1 0.9297 0] EVENT TICK
  ;[1 1 1] Spawn health when die
  (`/Engine/EditorBlueprintResources/StandardMacros.IsValid` _returnvalue
    (:`Is Valid`
      (set `self.ActorLastLocation` (`self.K2_GetActorLocation` _returnvalue))
      (`|ExecutionSequence`
        (:`then_0`
          (if (`self.B3_IsBuilding`)
            (`self.ChainBuild`)
            (else
              (`self.B3_SetHoloTransform`))))
        (:`then_1`
          ;[1 1 1] InputDetection
          (`|ExecutionSequence`
            (:`then_0`)
            (:`then_1`
              (if (== (`self.GetOwner`) (`GameplayStatics.GetPlayerPawn` 0))
                (`|ExecutionSequence`
                  (:`then_0`
                    (if (`PlayerController.IsInputKeyDown` (`GameplayStatics.GetPlayerController` 0) "X")
                      (`|ExecutionSequence`
                        (:`then_0`
                          (`/Engine/EditorBlueprintResources/StandardMacros.DoOnce` false :!label _label
                            (:`Completed`
                              (`self.B3KeyXPress`))))
                        (:`then_1`
                          (goto _label_2 :!via `Reset`)))
                      (else
                        (`|ExecutionSequence`
                          (:`then_0`
                            (`/Engine/EditorBlueprintResources/StandardMacros.DoOnce` true :!label _label_2))
                          (:`then_1`
                            (goto _label :!via `Reset`))))))
                  (:`then_1`
                    (if (or (`PlayerController.IsInputKeyDown` (`GameplayStatics.GetPlayerController` 0) "RightMouseButton") (`PlayerController.IsInputKeyDown` (`GameplayStatics.GetPlayerController` 0) "F") (`PlayerController.IsInputKeyDown` (`GameplayStatics.GetPlayerController` 0) "NumPadZero"))
                      (`|ExecutionSequence`
                        (:`then_0`
                          (`/Engine/EditorBlueprintResources/StandardMacros.DoOnce` false :!label _label_3
                            (:`Completed`
                              (`self.B3KeyBuildPress`))))
                        (:`then_1`
                          (goto _label_4 :!via `Reset`)))
                      (else
                        (`|ExecutionSequence`
                          (:`then_0`
                            (`/Engine/EditorBlueprintResources/StandardMacros.DoOnce` true :!label _label_4
                              (:`Completed`
                                (`self.B3KeyBuildRelease` false))))
                          (:`then_1`
                            (goto _label_3 :!via `Reset`))))))
                  (:`then_2`
                    (if (`PlayerController.IsInputKeyDown` (`GameplayStatics.GetPlayerController` 0) "C")
                      (`|ExecutionSequence`
                        (:`then_0`
                          (`/Engine/EditorBlueprintResources/StandardMacros.DoOnce` false :!label _label_5
                            (:`Completed`
                              (`self.B3KeyCPress`))))
                        (:`then_1`
                          (goto _label_6 :!via `Reset`)))
                      (else
                        (`|ExecutionSequence`
                          (:`then_0`
                            (`/Engine/EditorBlueprintResources/StandardMacros.DoOnce` true :!label _label_6))
                          (:`then_1`
                            (goto _label_5 :!via `Reset`))))))
                  (:`then_3`
                    (if (`PlayerController.IsInputKeyDown` (`GameplayStatics.GetPlayerController` 0) "V")
                      (`|ExecutionSequence`
                        (:`then_0`
                          (`/Engine/EditorBlueprintResources/StandardMacros.DoOnce` false :!label _label_7
                            (:`Completed`
                              (`self.B3KeyVPress`))))
                        (:`then_1`
                          (goto _label_8 :!via `Reset`)))
                      (else
                        (`|ExecutionSequence`
                          (:`then_0`
                            (`/Engine/EditorBlueprintResources/StandardMacros.DoOnce` true :!label _label_8))
                          (:`then_1`
                            (goto _label_7 :!via `Reset`)))))))))))))
    (:`Is Not Valid`
      ;;[1 1 1] Death
      (`/Engine/EditorBlueprintResources/StandardMacros.DoOnce` false
        (:`Completed`
          (`self.B3KeyBuildRelease` false)
          (`self.SetLifeSpan` (`self.B3_BP_Holos`) 0.01)
          (`self.SetLifeSpan` (`self.REF_HoloShape`) 0.01)
          (`self.SpawnHealth` (`self.ActorLastLocation`)))))))

(event `AnyInput`
  (`/Engine/EditorBlueprintResources/ActorMacros.Switch Has Authority`
    (:`Authority`
      (if (== (`self.GetOwner`) (`GameplayStatics.GetPlayerPawn` 0))
        (set `self.PlayerIndex` 0)
        (switch `/Game/RestrictedAssets/Tutorials/Lunar/Labu/E_LabuInput` (`self.Input`) :!label _label_9
          (:`NewEnumerator0`
            (`self.B1KeyPress`))
          (:`NewEnumerator1`
            (`self.B1KeyRelease`)))))
    (:`Remote`
      (`self.ClientRequest` (`Pawn.PlayerState` (`GameplayStatics.GetPlayerPawn` 0)) (`self.Input`)))))

(event `ClientRequest`
  (params (PlayerState :type "PlayerState Object Reference") (Selection :type "/Game/RestrictedAssets/Tutorials/Lunar/Labu/E_LabuInput Enum"))
  (set `self.Input` Selection)
  (`KismetSystemLibrary.PrintString` "ClientRequest" true true (struct :`G` 0.66 :`B` 1.0 :`A` 1.0) 99.0)
  (`/Engine/EditorBlueprintResources/ActorMacros.Switch Has Authority`
    (:`Authority`
      (for (_array_element _array_index) (`GameStateBase.PlayerArray` (`GameplayStatics.GetGameState`))
        (if (== _array_element PlayerState)
          (set `self.PlayerIndex` _array_index)))
      (goto _label_9))))

(event `B1KeyPress`
  (bind _build1_impactpoint (`self.Build1_ImpactPoint`))
  (bind _returnvalue (`GameplayStatics.GetPlayerCameraManager` (`self.PlayerIndex`)))
  (bind _returnvalue_2 (`PlayerCameraManager.GetCameraLocation` _returnvalue))
  (bind (_returnvalue_x _returnvalue_y) (`KismetMathLibrary.BreakVector` (`PlayerCameraManager.GetCameraLocation` (`GameplayStatics.GetPlayerCameraManager` (`self.PlayerIndex`)))))
  (bind _returnvalue_3 (`KismetMathLibrary.MakeRotFromZX` (`self.Build1_Normal`) (- (`KismetMathLibrary.MakeVector` _returnvalue_x _returnvalue_y (.z _build1_impactpoint)) _build1_impactpoint)))
  (bind _outhit (`KismetSystemLibrary.LineTraceSingle` :`Start` _returnvalue_2 :`End` (+ _returnvalue_2 (* (`self.GetActorForwardVector` _returnvalue) 10000.0)) :`TraceChannel` "TraceTypeQuery1" :`DrawTime` 5.0))
  (bind (_bblockinghit _binitialoverlap _time _location _impactpoint _normal) (`GameplayStatics.BreakHitResult` _outhit))
  (set `self.Build1_Normal` _normal)
  (set `self.Build1_ImpactPoint` _impactpoint)
  (set `self.Build1_IsBuilding` true)
  ;[1 1 1] ne  fonctionne pas
  ; useless?
  (set `self.Build1_BuildMouseINIT` (`self.GetInputAxisKeyValue`))
  (bind _returnvalue_4 (`|SpawnActorFromClass` "/Game/RestrictedAssets/Tutorials/Lunar/Labu/_ARCH/BP_BuildWall1.BP_BuildWall1_C" (`KismetMathLibrary.MakeTransform` (`self.Build1_ImpactPoint`) _returnvalue_3) "Undefined" "OverrideRootScale"))
  (set `self.Build1_CurrentBuildWall` _returnvalue_4)
  (bind _returnvalue_5 (`|SpawnActorFromClass` "/Game/RestrictedAssets/Tutorials/Lunar/Labu/_ARCH/BP_LunarCube_EditLabuBuild1.BP_LunarCube_EditLabuBuild1_C" (`KismetMathLibrary.MakeTransform` (`self.Build1_ImpactPoint`) _returnvalue_3 (0.1 0.1 0.1)) "Undefined" "OverrideRootScale"))
  (set `self.Build1_HoloCube` _returnvalue_5))

(event `B1KeyRelease`
  (bind _build1_holocube (`self.Build1_HoloCube`))
  (set `self.Build1_IsBuilding` false)
  (`self.K2_DestroyActor` (`self.Build1_CurrentBuildWall`))
  (`KismetSystemLibrary.PrintString` (`KismetStringLibrary.Concat_StrStr` "==============>" (`KismetSystemLibrary.GetDisplayName` _build1_holocube)) true true (struct :`G` 1.0 :`B` 0.035765 :`A` 1.0))
  (set `self.B1_NewCubeTransform` (`self.GetTransform` _build1_holocube))
  (`self.K2_DestroyActor` (`self.Build1_HoloCube`))
  (bind _returnvalue (`|SpawnActorFromClass` "/Game/RestrictedAssets/Tutorials/Lunar/Labu/_ARCH/BP_LunarCube_EditLabuBuild1.BP_LunarCube_EditLabuBuild1_C" (`self.B1_NewCubeTransform`) "Undefined" "OverrideRootScale"))
  (`/Game/RestrictedAssets/Tutorials/Lunar/Labu/_ARCH/BP_LunarCube_EditLabuBuild1.SetGoodMat` _returnvalue))

(event `B3KeyXPress`
  (set `self.B3_ShapeIndex` 0)
  (`self.B3_HideHolos` :!label _label_10)
  (`/Game/RestrictedAssets/Tutorials/Lunar/UI/UI_BuildCooldown.UISelectAShape` (`self.UI_BuildCooldown`) (`self.B3_ShapeIndex`) false)
  (if (`self.B3_IsBuilding`)
    (for _array_element (`self.B3_CurrentHolos`)
      (`/Game/RestrictedAssets/Tutorials/Lunar/Labu/BP_B3_Holos.ChangeAllShapes` _array_element (`self.B3_ShapeIndex`)))
    (else
      (`self.B3_ShowCurrentHolo` false))))

(event `B3KeyCPress`
  (set `self.B3_ShapeIndex` 1)
  (goto _label_10))

(event `B3KeyVPress`
  (set `self.B3_ShapeIndex` 2)
  (goto _label_10))

(event `B3KeyBPress`
  (set `self.B3_ShapeIndex` 3)
  (goto _label_10))

(event `B3KeyBuildPress`
  (bind _b3_cooldown (`self.B3_Cooldown`))
  ;[1 1 1] B3 Press
  (if (`self.B3_CanBuild`)
    (set `self.B3_CanBuild` false)
    (`|ExecutionSequence`
      (:`then_0`
        (`GameplayStatics.PlaySound2D` "/Game/RestrictedAssets/Tutorials/Lunar/Sound/SFX/BuildFirstTile/SFX_BuildFirstTile_Cue.SFX_BuildFirstTile_Cue")
        (`KismetSystemLibrary.Delay` 0.2)
        (`GameplayStatics.PlaySound2D` "/Game/RestrictedAssets/Tutorials/Lunar/Sound/SFX/SFX_BuilderReload_Cue.SFX_BuilderReload_Cue"))
      (:`then_1`
        (set `self.B3_IsBuilding` true)
        (`self.B3_HideHolos`)
        (set `self.B3_BuildUID` (`KismetStringLibrary.Conv_StringToName` (`KismetStringLibrary.Conv_IntToString` (`KismetMathLibrary.RandomInteger` 99999))))
        (`self.B3_SpawnTile` (`SceneComponent.K2_GetComponentToWorld` (`self.B3_GetCurrentShape`)))
        (`/Game/RestrictedAssets/Tutorials/Lunar/UI/UI_BuildCooldown.ShowBuilderLoading` (`self.UI_BuildCooldown`) _b3_cooldown)
        (`KismetSystemLibrary.Delay` _b3_cooldown)
        (set `self.B3_CanBuild` true)
        (if (not (`self.B3_IsBuilding`))
          (`self.B3_ShowCurrentHolo` true))))
    (else
      (`GameplayStatics.PlaySound2D` "/Game/RestrictedAssets/Tutorials/Lunar/Sound/SFX/SFX_CantBuild_Cue.SFX_CantBuild_Cue" 3.0))))

(event `B3KeyBuildRelease`
  (params (IsDead :type Boolean))
  ;[1 1 1] B3 Release
  (set `self.B3_IsBuilding` false)
  (for _array_element (`self.B3_CurrentHolos`)
    (`/Engine/EditorBlueprintResources/StandardMacros.IsValid` _array_element
      (:`Is Valid`
        (`/Game/RestrictedAssets/Tutorials/Lunar/Labu/BP_B3_Holos.KillAllHolo` _array_element))))
  (`KismetArrayLibrary.Array_Clear` (`self.B3_CurrentHolos`))
  (if (and (`self.B3_CanBuild`) (not IsDead))
    (`self.B3_ShowCurrentHolo` true)))

(event `BuildShape`
  (params (SpawnTransform :type "Transform Structure") (ShapeType :type Integer) (NewItem :type "Name (by ref)"))
  (bind _returnvalue (`|SpawnActorFromClass` "/Game/RestrictedAssets/Tutorials/Lunar/Labu/BP_B3_Shape.BP_B3_Shape_C" SpawnTransform "Undefined" "OverrideRootScale"))
  (`/Game/RestrictedAssets/Tutorials/Lunar/Labu/BP_B3_Shape.SetShape` _returnvalue NewItem ShapeType))

(event `SpawnHealth`
  (params (ActorLastLocation :type "Vector Structure"))
  (`|SpawnActorFromClass` "/Game/RestrictedAssets/Tutorials/Lunar/Labu/BP_HealthPack.BP_HealthPack_C" (`KismetMathLibrary.MakeTransform` (+ ActorLastLocation (0.0 0.0 50.0))) "Undefined" "OverrideRootScale"))

(fn `B3_GetCurrentShape`
  (returns (ReturnValue :type "SceneComponent Object Reference"))
  (bind _sm_holoslope_ref (`self.SM_HoloSlope_REF`))
  (return (select `int` (`self.B3_ShapeIndex`) :`0` (`self.SM_HoloWall_REF`) :`1` (`self.SM_HoloFloor_REF`) :`2` _sm_holoslope_ref :`3` _sm_holoslope_ref :!type "SceneComponent Object Reference")))

(fn `B3_HideHolos`
  (`SceneComponent.SetHiddenInGame` (`self.SM_HoloSlope_REF`) true false)
  (`SceneComponent.SetHiddenInGame` (`self.SM_HoloFloor_REF`) true false)
  (`SceneComponent.SetHiddenInGame` (`self.SM_HoloWall_REF`) true false))

(fn `B3_SetHoloTransform`
  (bind _returnvalue (`GameplayStatics.GetPlayerCharacter` 0))
  (bind _returnvalue_2 (`self.B3_GetCurrentShape`))
  (bind (_returnvalue_roll _returnvalue_pitch _returnvalue_yaw) (`KismetMathLibrary.BreakRotator` (`self.K2_GetActorRotation` _returnvalue)))
  (if (`self.B3_CanBuild`)
    (`/Engine/EditorBlueprintResources/StandardMacros.IsValid` _returnvalue_2
      (:`Is Valid`
        (`SceneComponent.K2_SetWorldLocationAndRotation` _returnvalue_2 (`KismetMathLibrary.MakeVector` (.x (+ (`self.K2_GetActorLocation` _returnvalue) (* (`self.GetActorForwardVector` _returnvalue) (select `int` (`self.B3_ShapeIndex`) :`0` 250.0 :`1` -10.0 :`2` 100.0 :`3` 300.0 :!type "Float (single-precision)")))) (.y (+ (`self.K2_GetActorLocation` _returnvalue) (* (`self.GetActorForwardVector` _returnvalue) (select `int` (`self.B3_ShapeIndex`) :`0` 250.0 :`1` -10.0 :`2` 100.0 :`3` 300.0 :!type "Float (single-precision)")))) (- (.z (+ (`self.K2_GetActorLocation` _returnvalue) (* (`self.GetActorForwardVector` _returnvalue) (select `int` (`self.B3_ShapeIndex`) :`0` 250.0 :`1` -10.0 :`2` 100.0 :`3` 300.0 :!type "Float (single-precision)")))) 110.151)) (`KismetMathLibrary.MakeRotator` 0.0 0.0 _returnvalue_yaw) false false)))))

(fn `B3_ShowCurrentHolo`
  (params (PlaySound :type Boolean))
  (`SceneComponent.SetHiddenInGame` (`self.B3_GetCurrentShape`) false false)
  (if PlaySound
    (`GameplayStatics.PlaySound2D` "/Game/RestrictedAssets/Tutorials/Lunar/Sound/SFX/SFX_BuilderReady_Cue.SFX_BuilderReady_Cue")))

(fn `B3_SpawnTile`
  (params (SpawnTransform :type "Transform Structure"))
  (bind _b3_bp_holos (`self.B3_BP_Holos`))
  (bind _returnvalue (`|SpawnActorFromClass` "/Game/RestrictedAssets/Tutorials/Lunar/Labu/BP_B3_Holos.BP_B3_Holos_C" SpawnTransform "Undefined" "OverrideRootScale"))
  (bind _output_get (set `self.B3_BP_Holos` _returnvalue))
  (`KismetArrayLibrary.Array_AddUnique` (`self.B3_CurrentHolos`) _output_get)
  (`/Game/RestrictedAssets/Tutorials/Lunar/Labu/BP_B3_Holos.SetHolos` (`self.B3_BP_Holos`) (`self.B3_ShapeIndex`))
  (`KismetArrayLibrary.Array_Add` (`Actor.Tags` _b3_bp_holos) (`self.B3_BuildUID`))
  (`/Game/RestrictedAssets/Tutorials/Lunar/Labu/BP_B3_Holos.CheckOverlaps` _b3_bp_holos))

(fn `Build1Press`
  (bind _returnvalue (`GameplayStatics.GetPlayerCameraManager` 0))
  (bind _build1_impactpoint (`self.Build1_ImpactPoint`))
  (bind _returnvalue_2 (`PlayerCameraManager.GetCameraLocation` _returnvalue))
  (bind (_returnvalue_x _returnvalue_y) (`KismetMathLibrary.BreakVector` (`PlayerCameraManager.GetCameraLocation` (`GameplayStatics.GetPlayerCameraManager` 0))))
  (bind _returnvalue_3 (`KismetMathLibrary.MakeRotFromZX` (`self.Build1_Normal`) (- (`KismetMathLibrary.MakeVector` _returnvalue_x _returnvalue_y (.z _build1_impactpoint)) _build1_impactpoint)))
  (bind _outhit (`KismetSystemLibrary.LineTraceSingle` :`Start` _returnvalue_2 :`End` (+ _returnvalue_2 (* (`self.GetActorForwardVector` _returnvalue) 10000.0)) :`TraceChannel` "TraceTypeQuery1" :`DrawTime` 5.0))
  (bind (_bblockinghit _binitialoverlap _time _location _impactpoint _normal) (`GameplayStatics.BreakHitResult` _outhit))
  (set `self.Build1_Normal` _normal)
  (set `self.Build1_ImpactPoint` _impactpoint)
  (bind _returnvalue_4 (`|SpawnActorFromClass` "/Game/RestrictedAssets/Tutorials/Lunar/Labu/_ARCH/BP_LunarCube_EditLabuBuild1.BP_LunarCube_EditLabuBuild1_C" (`KismetMathLibrary.MakeTransform` (`self.Build1_ImpactPoint`) _returnvalue_3 (0.1 0.1 0.1)) "Undefined" "OverrideRootScale"))
  (set `self.Build1_HoloCube` _returnvalue_4)
  (set `self.Build1_IsBuilding` true)
  ;[1 1 1] ne  fonctionne pas
  ; useless?
  (set `self.Build1_BuildMouseINIT` (`self.GetInputAxisKeyValue`))
  (bind _returnvalue_5 (`|SpawnActorFromClass` "/Game/RestrictedAssets/Tutorials/Lunar/Labu/_ARCH/BP_BuildWall1.BP_BuildWall1_C" (`KismetMathLibrary.MakeTransform` (`self.Build1_ImpactPoint`) _returnvalue_3) "Undefined" "OverrideRootScale"))
  (set `self.Build1_CurrentBuildWall` _returnvalue_5))

(fn `Build1Tick`
  (bind _returnvalue (`GameplayStatics.GetPlayerCameraManager` 0))
  (bind _build1_impactpoint (`self.Build1_ImpactPoint`))
  (bind _returnvalue_2 (`PlayerCameraManager.GetCameraLocation` _returnvalue))
  (bind (_returnvalue_x _returnvalue_y) (`KismetMathLibrary.BreakVector` (`PlayerCameraManager.GetCameraLocation` (`GameplayStatics.GetPlayerCameraManager` 0))))
  (bind _buildtarget (`/Game/RestrictedAssets/Tutorials/Lunar/Labu/_ARCH/BP_BuildWall1.BuildTarget` (`self.Build1_CurrentBuildWall`)))
  (bind (_relativelocation_x _relativelocation_y _relativelocation_z) (`KismetMathLibrary.BreakVector` (`SceneComponent.RelativeLocation` _buildtarget)))
  (bind _returnvalue_3 (`KismetMathLibrary.MakeRotFromZX` (`self.Build1_Normal`) (- (`KismetMathLibrary.MakeVector` _returnvalue_x _returnvalue_y (.z _build1_impactpoint)) _build1_impactpoint)))
  (if (`self.Build1_IsBuilding`)
    (bind _outhit (`KismetSystemLibrary.LineTraceSingle` :`Start` _returnvalue_2 :`End` (+ _returnvalue_2 (* (`self.GetActorForwardVector` _returnvalue) 10000.0)) :`TraceChannel` "TraceTypeQuery1" :`TraceColor` (struct :`G` 1.0 :`B` 1.0 :`A` 1.0) :`TraceHitColor` (struct :`R` 1.0 :`B` 0.930164 :`A` 1.0)))
    (`SceneComponent.K2_SetWorldLocation` _buildtarget (`.ImpactPoint` (`GameplayStatics.BreakHitResult` _outhit)) false false)
    (bind _output_get (set `self.CurrentScaleZ` (`KismetMathLibrary.FClamp` (* (select `bool` (> _relativelocation_z 0.1) :`false` 0.1 :`true` _relativelocation_z) 0.01) 0.1 10.0)))
    (bind _output_get_2 (set `self.CurrentScaleY` (`KismetMathLibrary.FClamp` (* (`KismetMathLibrary.Abs` _relativelocation_y) 0.02) 0.1 10.0)))
    ;[1 1 1] useless?
    (set `self.CurrentScaleX` (`KismetMathLibrary.FClamp` (* (`KismetMathLibrary.Abs` _relativelocation_x) 0.02) 0.1 10.0))
    (`/Engine/EditorBlueprintResources/ActorMacros.Switch Has Authority`
      (:`Authority`
        (`/Game/RestrictedAssets/Tutorials/Lunar/Labu/_ARCH/BP_LunarCube_EditLabuBuild1.Rescale` (`self.Build1_HoloCube`) (`KismetMathLibrary.MakeVector` _output_get_2 _output_get_2 _output_get))
        (`self.K2_SetActorRotation` (`self.Build1_CurrentBuildWall`) _returnvalue_3 false)
        (`self.K2_SetActorRotation` (`self.Build1_HoloCube`) _returnvalue_3 false)))))

(fn `ChainBuild`
  (bind _returnvalue (`GameplayStatics.GetPlayerCameraManager` 0))
  (bind _returnvalue_2 (`GameplayStatics.GetPlayerCharacter` 0))
  (bind _returnvalue_3 (`PlayerCameraManager.GetCameraLocation` _returnvalue))
  (bind _returnvalue_4 (`PlayerCameraManager.GetCameraLocation` (`GameplayStatics.GetPlayerCameraManager` 0)))
  (bind _returnvalue_5 (`KismetMathLibrary.ClampVectorSize` (`self.GetVelocity` _returnvalue_2) 0.0 100.0))
  (`|ExecutionSequence`
    (:`then_0`
      (bind (_outhit _returnvalue_6) (`KismetSystemLibrary.LineTraceSingle` :`Start` _returnvalue_3 :`End` (+ _returnvalue_3 (* (`self.GetActorForwardVector` _returnvalue) 750.0)) :`TraceChannel` "TraceTypeQuery1" :`DrawTime` 5.0))
      (if _returnvalue_6
        (`self.LineTraceActions` _outhit)))
    (:`then_1`
      (bind (_outhit_2 _returnvalue_7) (`KismetSystemLibrary.LineTraceSingle` :`Start` (+ _returnvalue_4 _returnvalue_5) :`End` (+ (+ _returnvalue_4 (* (`self.GetActorUpVector` _returnvalue_2) -500.0)) _returnvalue_5) :`TraceChannel` "TraceTypeQuery1" :`DrawTime` 5.0))
      (if _returnvalue_7
        (`self.LineTraceActions` _outhit_2)))))

(fn `FireShotOverride`
  (returns (ReturnValue :type Boolean))
  (return false))

(fn `GetOrCreateUI`
  ;[1 1 1] Erreur mais ça marche quand même alors...
  (bind _foundwidgets (`WidgetBlueprintLibrary.GetAllWidgetsOfClass` "/Game/RestrictedAssets/Tutorials/Lunar/UI/UI_BuildCooldown.UI_BuildCooldown_C"))
  (if (> (`KismetArrayLibrary.Array_Length` _foundwidgets) 0)
    (set `self.UI_BuildCooldown` (`KismetArrayLibrary.Array_Get` _foundwidgets))
    (else
      (bind _returnvalue (`|CreateWidget` "/Game/RestrictedAssets/Tutorials/Lunar/UI/UI_BuildCooldown.UI_BuildCooldown_C" (`GameplayStatics.GetPlayerController` 0)))
      (set `self.UI_BuildCooldown` _returnvalue)
      (`UserWidget.AddToViewport` (`self.UI_BuildCooldown`) 0))))

(fn `LineTraceActions`
  (params (Hit :type "HitResult Structure (by ref)"))
  (bind (_bblockinghit _binitialoverlap _time _location _impactpoint _normal _impactnormal _physmat _hitactor _hitcomponent) (`GameplayStatics.BreakHitResult` Hit))
  (bind _b3_nextspawntransform (`self.B3_NextSpawnTransform`))
  (bind (_returnvalue_location _returnvalue_rotation) (`KismetMathLibrary.BreakTransform` (`SceneComponent.K2_GetComponentToWorld` _hitcomponent)))
  (if (`ActorComponent.ComponentHasTag` _hitcomponent "holo")
    (set `self.B3_NextSpawnTransform` (`KismetMathLibrary.MakeTransform` _returnvalue_location _returnvalue_rotation))
    (`/Game/RestrictedAssets/Tutorials/Lunar/Labu/BP_B3_Holos.KillHoloShape` (cast `/Game/RestrictedAssets/Tutorials/Lunar/Labu/BP_B3_Holos` _hitactor :!pure true) _hitcomponent)
    (`self.B3_SpawnTile` _b3_nextspawntransform)
    (`GameplayStatics.PlaySoundAtLocation` "/Game/RestrictedAssets/Tutorials/Lunar/Sound/SFX/BuildNextTile/SFX_BuildNextTile_Cue.SFX_BuildNextTile_Cue" (.location _b3_nextspawntransform))))

(fn `UserConstructionScript`)