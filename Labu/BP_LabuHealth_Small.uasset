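; BP_LabuHealth_Small is a small health pickup that animates in place until it is taken.
; Each Tick spins HealthMesh around yaw and bobs it vertically with a sine of game time.
; It also calls the parent Tick and polls IsTaken, destroying the actor after a short delay once that returns true.
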(event `self.ReceiveTick`
  (params (DeltaSeconds :type "Float (single-precision)"))
  (`parent.ReceiveTick` DeltaSeconds)
  ;[1 1 1] rotate
  (`SceneComponent.K2_AddLocalRotation` (`self.Health Mesh`) (`KismetMathLibrary.MakeRotator` 0.0 0.0 (* DeltaSeconds 100.0)) false false)
  ;[1 1 1] bob
  (`SceneComponent.K2_SetRelativeLocation` (`self.Health Mesh`) (`KismetMathLibrary.MakeVector` 0.0 0.0 (* (`KismetMathLibrary.Sin` (* (`KismetSystemLibrary.GetGameTimeInSeconds`) 3.0)) 3.0)) false false)
  (bind _returnvalue (`self.IsTaken` null))
  (if _returnvalue
    (`KismetSystemLibrary.Delay` 0.5)
    (`self.K2_DestroyActor`)))

(fn `UserConstructionScript`)