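; Destructible build piece that SetShape orients and scales by shape type and tags with its build ID.
; Tick decays unreinforced step-0 pieces on authority; point and radial damage also drain life, scaled by reinforcement step.
; Repeated Reinforcement calls run down a cooldown, shown by a scaling sign, to raise the step up to max shield.
; Life drives a shared dynamic material across chunk meshes; at zero, particles spawn and the actor expires.
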(event `self.SM_LabuSlope_DM.OnComponentFracture`
  (params (HitPoint :type "Vector Structure (by ref)") (HitDirection :type "Vector Structure (by ref)"))
  ;[1 0 0] old
)

(event `self.ReceiveHit`
  (params (MyComp :type "PrimitiveComponent Object Reference") (Other :type "Actor Object Reference") (OtherComp :type "PrimitiveComponent Object Reference") (bSelfMoved :type Boolean) (HitLocation :type "Vector Structure") (HitNormal :type "Vector Structure") (NormalImpulse :type "Vector Structure") (Hit :type "HitResult Structure (by ref)"))
  ;[1 0 0] old
)

(event `self.ReceiveBeginPlay`
  ;[0.1148 1 0] BEGIN PLAY
  (`self.InitReinforcementCoolDown`)
  (bind _returnvalue (`KismetMaterialLibrary.CreateDynamicMaterialInstance` "/Game/RestrictedAssets/Tutorials/Lunar/Labu/M_ConcreteSlab_LabuEdit.M_ConcreteSlab_LabuEdit"))
  (set `self.INST_M_Concrete` _returnvalue)
  (for _array_element (`SceneComponent.GetChildrenComponents` (`self.Scene`) false)
    (bind _asstatic_mesh_component (cast `StaticMeshComponent` _array_element))
    (`KismetArrayLibrary.Array_AddUnique` (`self.SM_Chunks`) _asstatic_mesh_component)
    (`PrimitiveComponent.SetMaterial` _asstatic_mesh_component 0 (`self.INST_M_Concrete`))))

(event `self.ReceiveTick`
  (params (DeltaSeconds :type "Float (single-precision)"))
  ;[1 0.8632 0] EVENT TICK
  (`self.Alive`
    (:`True`
      (`self.UpdateReinforcementSign`)
      (`self.ReduceLifeAlongTime`)
      (`self.TestLifeToDestroy`))))

(event `SetShape`
  (params (BuildUID :type "Name (by ref)") (ShapeType :type Integer))
  (bind _scene (`self.Scene`))
  (bind _shapetype (`self.ShapeType`))
  (set `self.ShapeType` ShapeType)
  (`SceneComponent.K2_SetRelativeRotation` _scene (select `int` _shapetype :`0` (struct :`Pitch` 90.0) :`1` (struct) :`2` (struct :`Pitch` 26.51) :!type "Rotator Structure") false false)
  (`SceneComponent.SetRelativeScale3D` _scene (select `int` _shapetype :`0` (1.0 1.0 0.5) :`1` (1.0 1.0 1.0) :`2` (1.12 1.0 0.5) :!type "Vector Structure"))
  (`SceneComponent.K2_SetRelativeLocation` (`self.Scene`) (select `int` _shapetype :`0` (-12.5 0.0 0.0) :`1` (0.0 0.0 0.0) :`2` (0.0 0.0 0.0) :!type "Vector Structure") false false)
  (`KismetArrayLibrary.Array_Add` (`self.Tags`) BuildUID))

(event `self.ReceivePointDamage`
  (params (Damage :type "Float (single-precision)") (DamageType :type "DamageType Object Reference") (HitLocation :type "Vector Structure") (HitNormal :type "Vector Structure") (HitComponent :type "PrimitiveComponent Object Reference") (BoneName :type Name) (ShotFromDirection :type "Vector Structure") (InstigatedBy :type "Controller Object Reference") (DamageCauser :type "Actor Object Reference") (HitInfo :type "HitResult Structure (by ref)"))
  (`self.Alive`
    (:`True`
      (`self.RemoveLife` Damage))))

(event `self.ReceiveRadialDamage`
  (params (DamageReceived :type "Float (single-precision)") (DamageType :type "DamageType Object Reference") (Origin :type "Vector Structure") (HitInfo :type "HitResult Structure (by ref)") (InstigatedBy :type "Controller Object Reference") (DamageCauser :type "Actor Object Reference"))
  (`self.Alive`
    (:`True`
      (`self.RemoveLife` DamageReceived))))

(event `LifeVisualFeedback`
  (for _array_element (`self.SM_Chunks`)
    (`MeshComponent.SetScalarParameterValueOnMaterials` _array_element "ZeroPVRed" (/ (`self.NewLife`) 100.0))))

(event `Destroy`
  (`GameplayStatics.SpawnEmitterAtLocation` "/Game/RestrictedAssets/Tutorials/Lunar/Corentin/DestructCube/PS_Destruct.PS_Destruct" (`SceneComponent.K2_GetComponentLocation` (`self.TempEmitterLoc`)))
  (`self.SetLifeSpan` 0.01))

(event `Reinforcement`
  (`self.Alive`
    (:`True`
      (if (not (`self.IsMaxShield`))
        (set `self.IsBeingReinforced` true)
        (`self.ReduceCoolDown`)
        ;[1 1 1] cooldown stop reinforcement
        (`TimelineComponent.SetTimelineLength` (`self.StopRCoolDown`) 1.0)
        (`Timeline|StopRCoolDown` :!via `PlayFromStart`
          (:`Finished`
            (set `self.IsBeingReinforced` false)))))))

(fn `InitReinforcementCoolDown`
  (set `self.ReinforcementCoolDown` (select `int` (`self.Step`) :`0` (`self.INIT_Step0to1_RCoolDown`) :`1` (`self.INIT_Step1yo2_RCoolDown`))))

(fn `OnRep_ShapeType`)

(fn `ReduceCoolDown`
  (bind _output_get (set `self.ReinforcementCoolDown` (- (`self.ReinforcementCoolDown`) (`GameplayStatics.GetWorldDeltaSeconds`))))
  (if (<= _output_get 0.0)
    (switch `int` (`self.Step`)
      (:`0`
        (set `self.Step` 1)
        (`self.InitReinforcementCoolDown`))
      (:`1`
        (set `self.Step` 2)
        (set `self.IsMaxShield` true)
        (set `self.IsBeingReinforced` false)))))

(fn `ReduceLifeAlongTime`
  (if (== (`self.Step`) 0)
    (`/Engine/EditorBlueprintResources/ActorMacros.Switch Has Authority`
      (:`Authority`
        (if (not (`self.IsBeingReinforced`))
          (`self.RemoveLife` (* (`GameplayStatics.GetWorldDeltaSeconds`) 10.0)))))))

(fn `RemoveLife`
  (params (LifeToBeRemoved :type "Float (double-precision)"))
  (set `self.NewLife` (- (`self.NewLife`) (* LifeToBeRemoved (select `int` (`self.Step`) :`0` 2.0 :`1` 1.0 :`2` 0.5 :!type "Float (single-precision)")))))

(fn `TestLifeToDestroy`
  (if (<= (`self.NewLife`) 0.0)
    (`/Engine/EditorBlueprintResources/StandardMacros.DoOnce` false
      (:`Completed`
        (set `self.IsActive` false)
        (`self.Destroy`)))
    (else
      (`self.LifeVisualFeedback`))))

(fn `UpdateReinforcementSign`
  (bind _returnvalue (+ (`self.ReinforcementCoolDown`) (`GameplayStatics.GetWorldDeltaSeconds`)))
  (bind _returnvalue_2 (select `int` (`self.Step`) :`0` (`self.INIT_Step0to1_RCoolDown`) :`1` (`self.INIT_Step1yo2_RCoolDown`)))
  (bind _returnvalue_3 (>= _returnvalue _returnvalue_2))
  (if (`self.IsBeingReinforced`)
    (`SceneComponent.SetHiddenInGame` (`self.TempSign`) false false)
    (elif (< (`self.Step`) 2)
      ;[1 1 1] BackUpCoolDown
      (set `self.ReinforcementCoolDown` (select `bool` _returnvalue_3 :`false` _returnvalue :`true` _returnvalue_2))
      (if _returnvalue_3
        (`SceneComponent.SetHiddenInGame` (`self.TempSign`) true false :!label _label))
      (else
        (goto _label))))
  (`SceneComponent.SetWorldScale3D` (`self.ReinforcementSignAnchor`) (`KismetMathLibrary.MakeVector` (- 1.0 (/ (`self.ReinforcementCoolDown`) (select `int` (`self.Step`) :`0` (`self.INIT_Step0to1_RCoolDown`) :`1` (`self.INIT_Step1yo2_RCoolDown`)))) 1.0 1.0)))

(fn `UserConstructionScript`)