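; BP_LabuBuilder1 is a prototype building tool with two main methods, driven by key polling on Tick.
; Holding LeftAlt in BuildMode spawns a camera-traced holo cube and helper wall; Tick scales and orients the cube until release commits it.
; X, C, V or B select a shape hologram ahead of the player, and right mouse stamps it as a detached, collidable mesh.
; An older block-scaling path remains on Tick, but its spawn logic is unwired.
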(event `self.ReceiveTick`
  (params (DeltaSeconds :type "Float (single-precision)"))
  (bind _returnvalue (`self.B3_GetCurrentShape`))
  (bind _returnvalue_2 (`GameplayStatics.GetPlayerCharacter` 0))
  (bind (_blocorigin_x _blocorigin_y _blocorigin_z) (`KismetMathLibrary.BreakVector` (`self.BlocOrigin`)))
  (bind _returnvalue_3 (`GameplayStatics.GetPlayerCameraManager` (`self.PlayerIndex`)))
  (bind (_returnvalue_x _returnvalue_y) (`KismetMathLibrary.BreakVector` (`self.GetActorScale3D` (`self.Bloc`))))
  (bind (_returnvalue_roll _returnvalue_pitch _returnvalue_yaw) (`KismetMathLibrary.BreakRotator` (`self.K2_GetActorRotation` _returnvalue_2)))
  (bind (_returnvalue_x_2 _returnvalue_y_2 _returnvalue_z) (`KismetMathLibrary.BreakVector` (+ (`PlayerCameraManager.GetCameraLocation` _returnvalue_3) (* (`KismetMathLibrary.GetForwardVector` (`PlayerCameraManager.GetCameraRotation` _returnvalue_3)) (`self.RayDist`)))))
  (`|ExecutionSequence`
    (:`then_0`
      (`/Engine/EditorBlueprintResources/ActorMacros.Switch Has Authority`
        (:`Authority`
          _)
        (:`Remote`
          _))
      (if (`self.BuildMode?`)
        (if (`self.BlocXY`)
          (set `/Game/RestrictedAssets/Tutorials/Lunar/BP_LunarCube.Scale` (`KismetMathLibrary.MakeVector` (`KismetMathLibrary.FClamp` (/ (- _blocorigin_x _returnvalue_x_2) 100.0) -15.0 15.0) (`KismetMathLibrary.FClamp` (/ (- _returnvalue_y_2 _blocorigin_y) -100.0) -15.0 15.0)) (`self.Bloc`))
          (elif (`self.BlocZ`)
            (set `/Game/RestrictedAssets/Tutorials/Lunar/BP_LunarCube.Scale` (`KismetMathLibrary.MakeVector` _returnvalue_x _returnvalue_y (`KismetMathLibrary.FClamp` (/ (- _returnvalue_z _blocorigin_z) 75.0) -10.0 10.0)) (`self.Bloc`))))))
    (:`then_1`
      (`|ExecutionSequence`
        (:`then_0`
          (if (`self.B3ShowHolo`)
            (`KismetSystemLibrary.PrintString` (`KismetSystemLibrary.GetDisplayName` _returnvalue))
            (`SceneComponent.K2_SetWorldLocationAndRotation` _returnvalue (`KismetMathLibrary.MakeVector` (.x (+ (`self.K2_GetActorLocation` _returnvalue_2) (* (`self.GetActorForwardVector` _returnvalue_2) 300.0))) (.y (+ (`self.K2_GetActorLocation` _returnvalue_2) (* (`self.GetActorForwardVector` _returnvalue_2) 300.0))) (- (.z (+ (`self.K2_GetActorLocation` _returnvalue_2) (* (`self.GetActorForwardVector` _returnvalue_2) 300.0))) 110.151)) (`KismetMathLibrary.MakeRotator` 0.0 0.0 _returnvalue_yaw) false false)))
        (:`then_1`
          ;[1 1 1] Build 1 Tick
          (`self.Build1Tick`))))
    (:`then_2`
      (`|ExecutionSequence`
        (:`then_0`
          (if (`PlayerController.IsInputKeyDown` (`GameplayStatics.GetPlayerController` 0) "LeftAlt")
            (`|ExecutionSequence`
              (:`then_0`
                (`/Engine/EditorBlueprintResources/StandardMacros.DoOnce` false :!label _label
                  (:`Completed`
                    (`self.B1KeyPress`))))
              (:`then_1`
                (goto _label_2 :!via `Reset`)))
            (else
              (`|ExecutionSequence`
                (:`then_0`
                  (`/Engine/EditorBlueprintResources/StandardMacros.DoOnce` true :!label _label_2
                    (:`Completed`
                      (`self.B1KeyRelease`))))
                (:`then_1`
                  (goto _label :!via `Reset`))))))
        (:`then_1`
          (if (`PlayerController.IsInputKeyDown` (`GameplayStatics.GetPlayerController` 0) "X")
            (`|ExecutionSequence`
              (:`then_0`
                (`/Engine/EditorBlueprintResources/StandardMacros.DoOnce` false :!label _label_3
                  (:`Completed`
                    (`self.B3KeyXPress`))))
              (:`then_1`
                (goto _label_4 :!via `Reset`)))
            (else
              (`|ExecutionSequence`
                (:`then_0`
                  (`/Engine/EditorBlueprintResources/StandardMacros.DoOnce` true :!label _label_4))
                (:`then_1`
                  (goto _label_3 :!via `Reset`))))))
        (:`then_2`
          (if (`PlayerController.IsInputKeyDown` (`GameplayStatics.GetPlayerController` 0) "RightMouseButton")
            (`|ExecutionSequence`
              (:`then_0`
                (`/Engine/EditorBlueprintResources/StandardMacros.DoOnce` false :!label _label_5
                  (:`Completed`
                    (`self.B3KeyBuildPress`))))
              (:`then_1`
                (goto _label_6 :!via `Reset`)))
            (else
              (`|ExecutionSequence`
                (:`then_0`
                  (`/Engine/EditorBlueprintResources/StandardMacros.DoOnce` true :!label _label_6))
                (:`then_1`
                  (goto _label_5 :!via `Reset`))))))
        (:`then_3`
          (if (`PlayerController.IsInputKeyDown` (`GameplayStatics.GetPlayerController` 0) "C")
            (`|ExecutionSequence`
              (:`then_0`
                (`/Engine/EditorBlueprintResources/StandardMacros.DoOnce` false :!label _label_7
                  (:`Completed`
                    (`self.B3KeyCPress`))))
              (:`then_1`
                (goto _label_8 :!via `Reset`)))
            (else
              (`|ExecutionSequence`
                (:`then_0`
                  (`/Engine/EditorBlueprintResources/StandardMacros.DoOnce` true :!label _label_8))
                (:`then_1`
                  (goto _label_7 :!via `Reset`))))))
        (:`then_4`
          (if (`PlayerController.IsInputKeyDown` (`GameplayStatics.GetPlayerController` 0) "V")
            (`|ExecutionSequence`
              (:`then_0`
                (`/Engine/EditorBlueprintResources/StandardMacros.DoOnce` false :!label _label_9
                  (:`Completed`
                    (`self.B3KeyVPress`))))
              (:`then_1`
                (goto _label_10 :!via `Reset`)))
            (else
              (`|ExecutionSequence`
                (:`then_0`
                  (`/Engine/EditorBlueprintResources/StandardMacros.DoOnce` true :!label _label_10))
                (:`then_1`
                  (goto _label_9 :!via `Reset`))))))
        (:`then_5`
          (if (`PlayerController.IsInputKeyDown` (`GameplayStatics.GetPlayerController` 0) "B")
            (`|ExecutionSequence`
              (:`then_0`
                (`/Engine/EditorBlueprintResources/StandardMacros.DoOnce` false :!label _label_11
                  (:`Completed`
                    (`self.B3KeyBPress`))))
              (:`then_1`
                (goto _label_12 :!via `Reset`)))
            (else
              (`|ExecutionSequence`
                (:`then_0`
                  (`/Engine/EditorBlueprintResources/StandardMacros.DoOnce` true :!label _label_12))
                (:`then_1`
                  (goto _label_11 :!via `Reset`))))))))))

(event `B1KeyRelease`
  (`KismetSystemLibrary.PrintString` "Release")
  (set `self.Build1_IsBuilding` false)
  (`self.K2_DestroyActor` (`self.Build1_CurrentBuildWall`))
  (`/Game/RestrictedAssets/Tutorials/Lunar/Labu/BP_LunarCube_EditLabuBuild1.SetGoodMat` (`self.Build1_HoloCube`)))

(event `B1KeyPress`
  (`KismetSystemLibrary.PrintString` "Press")
  (`/Engine/EditorBlueprintResources/ActorMacros.Switch Has Authority`
    (:`Authority`
      (if (== (`self.GetOwner`) (`GameplayStatics.GetPlayerPawn` 0))
        (set `self.PlayerIndex` 0)
        (if (`self.End?`) :!label _label_13
          _
          (elif (`self.BuildMode?`)
            (`KismetSystemLibrary.PrintString` "BuildMode")
            ;[1 1 1] Build 1 Press
            (`self.Build1Press`)))))
    (:`Remote`
      (`self.ClientRequest` (`Pawn.PlayerState` (`GameplayStatics.GetPlayerPawn` 0))))))

(event `ClientRequest`
  (params (PlayerState :type "PlayerState Object Reference"))
  (`KismetSystemLibrary.PrintString` "cliReq")
  (`/Engine/EditorBlueprintResources/ActorMacros.Switch Has Authority`
    (:`Authority`
      (for (_array_element _array_index) (`GameStateBase.PlayerArray` (`GameplayStatics.GetGameState`))
        (if (== _array_element PlayerState)
          (set `self.PlayerIndex` _array_index)))
      (goto _label_13))))

(event `B3KeyXPress`
  (`self.B3_HideHolos`)
  (set `self.B3_ShapeIndex` 0)
  (`SceneComponent.SetHiddenInGame` (`self.B3_GetCurrentShape`) false false :!label _label_14))

(event `B3KeyCPress`
  (`self.B3_HideHolos`)
  (set `self.B3_ShapeIndex` 1)
  (goto _label_14))

(event `B3KeyVPress`
  (`self.B3_HideHolos`)
  (set `self.B3_ShapeIndex` 2)
  (goto _label_14))

(event `B3KeyBPress`
  (`self.B3_HideHolos`)
  (set `self.B3_ShapeIndex` 3)
  (goto _label_14))

(event `B3KeyBuildPress`
  (bind _b3_arrow (`self.B3_Arrow`))
  (bind _b3_addedsm (`self.B3_AddedSM`))
  (bind _returnvalue (`SceneComponent.GetRelativeTransform` _b3_arrow))
  (`SceneComponent.K2_SetWorldTransform` _b3_arrow (`SceneComponent.K2_GetComponentToWorld` (`self.B3_GetCurrentShape`)) false false)
  (switch `int` (`self.B3_ShapeIndex`)
    (:`0`
      (bind _returnvalue_2 (`AddComponent|NODE_AddStaticMeshComponent-5` :`RelativeTransform` _returnvalue))
      (set `self.B3_AddedSM` _returnvalue_2))
    (:`1`
      (bind _returnvalue_3 (`AddComponent|NODE_AddStaticMeshComponent-4` :`RelativeTransform` _returnvalue))
      (set `self.B3_AddedSM` _returnvalue_3))
    (:`2`
      (bind _returnvalue_4 (`AddComponent|NODE_AddStaticMeshComponent-2` :`RelativeTransform` _returnvalue))
      (set `self.B3_AddedSM` _returnvalue_4))
    (:`3`
      (bind _returnvalue_5 (`AddComponent|NODE_AddStaticMeshComponent-6` :`RelativeTransform` _returnvalue))
      (set `self.B3_AddedSM` _returnvalue_5)))
  (`PrimitiveComponent.SetCollisionEnabled` _b3_addedsm "QueryAndPhysics")
  (`PrimitiveComponent.SetCollisionResponseToAllChannels` _b3_addedsm "ECR_Block")
  (`PrimitiveComponent.SetMaterial` _b3_addedsm 0 "/Game/RestrictedAssets/Tutorials/Materials/M_Tut_Environment_Wall_C.M_Tut_Environment_Wall_C")
  (`SceneComponent.DetachFromParent` _b3_addedsm true true))

(fn `B3_GetCurrentShape`
  (returns (ReturnValue :type "SceneComponent Object Reference"))
  (return (select `int` (`self.B3_ShapeIndex`) :`0` (`self.SM_Wall`) :`1` (`self.SM_Floor`) :`2` (`self.SM_Slope`) :`3` null :!type "SceneComponent Object Reference")))

(fn `B3_HideHolos`
  (set `self.B3ShowHolo` true)
  (`SceneComponent.SetHiddenInGame` (`self.SM_Slope`) true false)
  (`SceneComponent.SetHiddenInGame` (`self.SM_Floor`) true false)
  (`SceneComponent.SetHiddenInGame` (`self.SM_Wall`) true false))

(fn `Build1Press`
  (bind _returnvalue (`GameplayStatics.GetPlayerCameraManager` 0))
  (bind _build1_impactpoint (`self.Build1_ImpactPoint`))
  (bind _returnvalue_2 (`PlayerCameraManager.GetCameraLocation` _returnvalue))
  (bind (_returnvalue_x _returnvalue_y) (`KismetMathLibrary.BreakVector` (`PlayerCameraManager.GetCameraLocation` (`GameplayStatics.GetPlayerCameraManager` 0))))
  (bind _returnvalue_3 (`KismetMathLibrary.MakeRotFromZX` (`self.Build1_Normal`) (- (`KismetMathLibrary.MakeVector` _returnvalue_x _returnvalue_y (.z _build1_impactpoint)) _build1_impactpoint)))
  (bind _outhit (`KismetSystemLibrary.LineTraceSingle` :`Start` _returnvalue_2 :`End` (+ _returnvalue_2 (* (`self.GetActorForwardVector` _returnvalue) 10000.0)) :`TraceChannel` "TraceTypeQuery1" :`DrawTime` 5.0))
  (bind (_bblockinghit _binitialoverlap _time _location _impactpoint _normal) (`GameplayStatics.BreakHitResult` _outhit))
  (set `self.Build1_Normal` _normal)
  (set `self.Build1_ImpactPoint` _impactpoint)
  (bind _returnvalue_4 (`|SpawnActorFromClass` "/Game/RestrictedAssets/Tutorials/Lunar/Labu/BP_LunarCube_EditLabuBuild1.BP_LunarCube_EditLabuBuild1_C" (`KismetMathLibrary.MakeTransform` (`self.Build1_ImpactPoint`) _returnvalue_3 (0.1 0.1 0.1)) "Undefined" "OverrideRootScale"))
  (set `self.Build1_HoloCube` _returnvalue_4)
  (set `self.Build1_IsBuilding` true)
  ;[1 1 1] ne  fonctionne pas
  ; useless?
  (set `self.Build1_BuildMouseINIT` (`self.GetInputAxisKeyValue`))
  (bind _returnvalue_5 (`|SpawnActorFromClass` "/Game/RestrictedAssets/Tutorials/Lunar/Labu/BP_BuildWall1.BP_BuildWall1_C" (`KismetMathLibrary.MakeTransform` (`self.Build1_ImpactPoint`) _returnvalue_3) "Undefined" "OverrideRootScale"))
  (set `self.Build1_CurrentBuildWall` _returnvalue_5))

(fn `Build1Tick`
  (bind _returnvalue (`GameplayStatics.GetPlayerCameraManager` 0))
  (bind _build1_impactpoint (`self.Build1_ImpactPoint`))
  (bind _returnvalue_2 (`PlayerCameraManager.GetCameraLocation` _returnvalue))
  (bind (_returnvalue_x _returnvalue_y) (`KismetMathLibrary.BreakVector` (`PlayerCameraManager.GetCameraLocation` (`GameplayStatics.GetPlayerCameraManager` 0))))
  (bind _buildtarget (`/Game/RestrictedAssets/Tutorials/Lunar/Labu/BP_BuildWall1.BuildTarget` (`self.Build1_CurrentBuildWall`)))
  (bind (_relativelocation_x _relativelocation_y _relativelocation_z) (`KismetMathLibrary.BreakVector` (`SceneComponent.RelativeLocation` _buildtarget)))
  (bind _returnvalue_3 (`KismetMathLibrary.MakeRotFromZX` (`self.Build1_Normal`) (- (`KismetMathLibrary.MakeVector` _returnvalue_x _returnvalue_y (.z _build1_impactpoint)) _build1_impactpoint)))
  (if (`self.Build1_IsBuilding`)
    (bind _outhit (`KismetSystemLibrary.LineTraceSingle` :`Start` _returnvalue_2 :`End` (+ _returnvalue_2 (* (`self.GetActorForwardVector` _returnvalue) 10000.0)) :`TraceChannel` "TraceTypeQuery1" :`TraceColor` (struct :`G` 1.0 :`B` 1.0 :`A` 1.0) :`TraceHitColor` (struct :`R` 1.0 :`B` 0.930164 :`A` 1.0)))
    (`SceneComponent.K2_SetWorldLocation` _buildtarget (`.ImpactPoint` (`GameplayStatics.BreakHitResult` _outhit)) false false)
    (bind _output_get (set `self.CurrentScaleZ` (`KismetMathLibrary.FClamp` (* (select `bool` (> _relativelocation_z 0.1) :`false` 0.1 :`true` _relativelocation_z) 0.01) 0.1 10.0)))
    (bind _output_get_2 (set `self.CurrentScaleY` (`KismetMathLibrary.FClamp` (* (`KismetMathLibrary.Abs` _relativelocation_y) 0.02) 0.1 10.0)))
    ;[1 1 1] useless?
    (set `self.CurrentScaleX` (`KismetMathLibrary.FClamp` (* (`KismetMathLibrary.Abs` _relativelocation_x) 0.02) 0.1 10.0))
    (`self.SetActorRelativeScale3D` (`self.Build1_HoloCube`) (`KismetMathLibrary.MakeVector` _output_get_2 _output_get_2 _output_get))
    (`self.K2_SetActorRotation` (`self.Build1_CurrentBuildWall`) _returnvalue_3 false)
    (`self.K2_SetActorRotation` (`self.Build1_HoloCube`) _returnvalue_3 false)))

(fn `FireShotOverride`
  (returns (ReturnValue :type Boolean))
  (return false))

(fn `UserConstructionScript`)