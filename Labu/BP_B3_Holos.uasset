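; BP_B3_Holos is a building-piece actor holding holographic placement previews for wall, floor, slope and ramp shapes.
; The construction script groups the hologram meshes by shape, and SetHolos reveals the selected group with query-only collision that blocks Visibility.
; CheckOverlaps destroys holograms overlapping another actor whose first tag matches its own.
; Other events destroy one or all holograms, or switch every hologram's mesh and translucent material.
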(event `CheckOverlaps`
  (for _array_element (`self.AllHolos`)
    (`/Engine/EditorBlueprintResources/StandardMacros.IsValid` _array_element
      (:`Is Valid`
        (set `self.CurrentTestedHolo` _array_element)
        (for _array_element_2 (`PrimitiveComponent.GetOverlappingComponents` (`self.CurrentTestedHolo`))
          (`/Engine/EditorBlueprintResources/StandardMacros.IsValid` _array_element_2
            (:`Is Valid`
              (set `self.CurrentOverlappingComponent` _array_element_2)
              (set `self.CurrentOwner` (`ActorComponent.GetOwner` (`self.CurrentOverlappingComponent`)))
              (if (!= (`self.CurrentOwner`) self)
                (if (== (`KismetArrayLibrary.Array_Get` (`self.Tags`)) (`KismetArrayLibrary.Array_Get` (`Actor.Tags` (`self.CurrentOwner`))))
                  (set `self.NeedDestroyTestedShape` true)
                  (break))))))
        (if (`self.NeedDestroyTestedShape`)
          (`ActorComponent.K2_DestroyComponent` (`self.CurrentTestedHolo`))
          (set `self.NeedDestroyTestedShape` false))))))

(event `SetHolos`
  (params (ShapeType :type Integer))
  (set `self.ShapeType` ShapeType)
  (`self.ShowCurrentHolos`))

(event `KillHoloShape`
  (params (A :type "Object Object Reference"))
  (for _array_element (`self.AllHolos`)
    (if (== _array_element A)
      (`ActorComponent.K2_DestroyComponent` _array_element))))

(event `KillAllHolo`
  (for _array_element (`self.AllHolos`)
    (`/Engine/EditorBlueprintResources/StandardMacros.IsValid` _array_element
      (:`Is Valid`
        (`ActorComponent.K2_DestroyComponent` _array_element)))))

(event `ChangeAllShapes`
  (params (NewParam :type Integer))
  (for _array_element (`self.AllHolos`)
    (`/Engine/EditorBlueprintResources/StandardMacros.IsValid` _array_element
      (:`Is Valid`
        (`StaticMeshComponent.SetStaticMesh` _array_element (select `int` NewParam :`0` "/Game/RestrictedAssets/Tutorials/Lunar/Labu/SM_Wall.SM_Wall" :`1` "/Game/RestrictedAssets/Tutorials/Lunar/Labu/SM_Floor.SM_Floor" :`2` "/Game/RestrictedAssets/Tutorials/Lunar/Labu/OLD_SM_Slope2.OLD_SM_Slope2" :`3` "/Game/RestrictedAssets/Tutorials/Lunar/Labu/_ARCH/SM_Ramp.SM_Ramp" :!type "StaticMesh Object Reference"))
        (`PrimitiveComponent.SetMaterial` _array_element 0 (select `int` NewParam :`0` "/Game/RestrictedAssets/Tutorials/Lunar/Labu/M_Trans_Wall.M_Trans_Wall" :`1` "/Game/RestrictedAssets/Tutorials/Lunar/Labu/M_Trans_Floor.M_Trans_Floor" :`2` "/Game/RestrictedAssets/Tutorials/Lunar/Labu/M_Trans_Slope.M_Trans_Slope" :`3` "/Game/RestrictedAssets/Tutorials/Lunar/Labu/_ARCH/M_Trans_Ramp.M_Trans_Ramp" :!type "MaterialInterface Object Reference"))))))

(fn `ShowCurrentHolos`
  (for _array_element (`self.AllHolos`)
    (`SceneComponent.SetHiddenInGame` _array_element true false))
  (`KismetArrayLibrary.Array_Clear` (`self.CurrentHolos`))
  (bind _output_get (set `self.CurrentHolos` (select `int` (`self.ShapeType`) :`0` (`self.WallHolos`) :`1` (`self.FloorHolos`) :`2` (`self.SlopeHolos`) :`3` (`self.RampHolos`))))
  (for _array_element_2 _output_get
    (`SceneComponent.SetHiddenInGame` _array_element_2 false false)
    (`PrimitiveComponent.SetCollisionEnabled` _array_element_2 "QueryOnly")
    (`PrimitiveComponent.SetCollisionResponseToChannel` _array_element_2 "ECC_Visibility" "ECR_Block")
    (`PrimitiveComponent.SetCollisionResponseToChannel` _array_element_2 "ECC_WorldStatic" "ECR_Overlap")
    (`PrimitiveComponent.SetCollisionResponseToChannel` _array_element_2 "ECC_WorldDynamic" "ECR_Overlap")))

(fn `UserConstructionScript`
  (bind _allholos (`self.AllHolos`))
  (set `self.FloorHolos` (`|MakeArray` (`self.SM_HoloFloor_T`) (`self.SM_HoloFloor_R`) (`self.SM_HoloFloor_L`) (`self.SM_HoloFloor_B`)))
  (set `self.WallHolos` (`|MakeArray` (`self.SM_HoloWall_R`) (`self.SM_HoloWall_T`) (`self.SM_HoloWall_B`) (`self.SM_HoloWall_L`)))
  (set `self.SlopeHolos` (`|MakeArray` (`self.SM_HoloSlope_T`) (`self.SM_HoloSlope_L`) (`self.SM_HoloSlope_R`) (`self.SM_HoloSlope_B`)))
  (set `self.RampHolos` (`|MakeArray` (`self.SM_HoloRamp_R`) (`self.SM_HoloRamp_B`) (`self.SM_HoloRamp_L`)))
  (`KismetArrayLibrary.Array_Append` _allholos (`self.WallHolos`))
  (`KismetArrayLibrary.Array_Append` _allholos (`self.FloorHolos`))
  (`KismetArrayLibrary.Array_Append` _allholos (`self.SlopeHolos`))
  (`KismetArrayLibrary.Array_Append` _allholos (`self.RampHolos`)))