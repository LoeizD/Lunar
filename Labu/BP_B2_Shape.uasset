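; Building shape actor that shows a wall, floor or slope mesh, with three holographic floor components (front, right, left), likely as placement previews.
; The construction script gathers the components into arrays, and SetShape picks the main mesh by type.
; CheckOverlaps destroys any component, main mesh included, overlapping another actor with the same first tag.
; Separate events remove one given hologram or all of them.
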(event `CheckOverlaps`
  (for _array_element (`self.AllShapes`)
    (`/Engine/EditorBlueprintResources/StandardMacros.IsValid` _array_element
      (:`Is Valid`
        (set `self.CurrentTestedShape` _array_element)
        (for _array_element_2 (`PrimitiveComponent.GetOverlappingComponents` (`self.CurrentTestedShape`))
          (`/Engine/EditorBlueprintResources/StandardMacros.IsValid` _array_element_2
            (:`Is Valid`
              (set `self.CurrentOverlappingComponent` _array_element_2)
              (set `self.CurrentOwner` (`ActorComponent.GetOwner` (`self.CurrentOverlappingComponent`)))
              (if (!= (`self.CurrentOwner`) self)
                (if (== (`KismetArrayLibrary.Array_Get` (`self.Tags`)) (`KismetArrayLibrary.Array_Get` (`Actor.Tags` (`self.CurrentOwner`))))
                  (`|ExecutionSequence`
                    (:`then_0`
                      (set `self.NeedDestroyTestedShape` true))
                    (:`then_1`
                      (break))))))))
        (if (`self.NeedDestroyTestedShape`)
          (`ActorComponent.K2_DestroyComponent` (`self.CurrentTestedShape`))
          (set `self.NeedDestroyTestedShape` false))))))

(event `SetShape`
  (params (ShapeType :type Integer))
  (set `self.ShapeType` ShapeType)
  (`StaticMeshComponent.SetStaticMesh` (`self.SM_Shape`) (select `int` (`self.ShapeType`) :`0` "/Game/RestrictedAssets/Tutorials/Lunar/Labu/SM_Wall.SM_Wall" :`1` "/Game/RestrictedAssets/Tutorials/Lunar/Labu/SM_Floor.SM_Floor" :`2` "/Game/RestrictedAssets/Tutorials/Lunar/Labu/SM_Slope2.SM_Slope2" :`3` "/Game/RestrictedAssets/Tutorials/Lunar/Labu/SM_Slope2.SM_Slope2" :!type "StaticMesh Object Reference")))

(event `KillHoloShape`
  (params (A :type "Object Object Reference"))
  (for _array_element (`self.FloorHolos`)
    (if (== _array_element A)
      (`ActorComponent.K2_DestroyComponent` _array_element))))

(event `KillAllHolo`
  (for _array_element (`self.FloorHolos`)
    (`/Engine/EditorBlueprintResources/StandardMacros.IsValid` _array_element
      (:`Is Valid`
        (`ActorComponent.K2_DestroyComponent` _array_element)))))

(fn `UserConstructionScript`
  (set `self.FloorHolos` (`|MakeArray` (`self.SM_HoloFloor_F`) (`self.SM_HoloFloor_R`) (`self.SM_HoloFloor_L`)))
  (set `self.AllShapes` (`|MakeArray` (`self.SM_HoloFloor_F`) (`self.SM_HoloFloor_L`) (`self.SM_HoloFloor_R`) (`self.SM_Shape`))))