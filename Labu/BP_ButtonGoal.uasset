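; Team goal button in an Unreal Tournament-based mode that ends the match when an opposing-team character touches it.
; The first valid overlap flags other-team buttons as pushed, zeroes their score, plays Redeemer explosion effects, calls EndMatch and freezes time via zero global dilation.
; UpdateScore pushes each team's score to the HUD on remote clients only.
; The construction script applies team color and positions the scoring-distance sign.
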(event `self.ReceiveActorBeginOverlap`
  (params (OtherActor :type "Actor Object Reference"))
  (bind _ascopy_default_character (cast `/Game/RestrictedAssets/Tutorials/Lunar/Labu/COPY_DefaultCharacter` OtherActor))
  (if (!= (`UTCharacter.GetTeamNum` _ascopy_default_character) (`self.Team`))
    (`/Engine/EditorBlueprintResources/StandardMacros.DoOnce` false
      (:`Completed`
        (cast `UTPlayerState` (`Pawn.PlayerState` _ascopy_default_character))
        (bind _outactors (`GameplayStatics.GetAllActorsOfClass` "BP_ButtonGoal_C"))
        (for _array_element _outactors
          (if (!= (`/Labu/BP_ButtonGoal.Team` _array_element) (`self.Team`))
            (set `/Labu/BP_ButtonGoal.ButtonPushed` true _array_element)
            (`self.UpdateScore` _array_element 0)))
        (`self.FxDeOuf` (`self.K2_GetActorLocation` _ascopy_default_character))
        (`KismetSystemLibrary.Delay` 0.2)
        ;[1 1 1] End
        (`GameMode.EndMatch` (cast `/Game/RestrictedAssets/Tutorials/Lunar/Labu/COPY_UTTeamGameMode` (`GameplayStatics.GetGameMode`) :!pure true))
        (`KismetSystemLibrary.Delay` 0.01)
        (`GameplayStatics.SetGlobalTimeDilation` 0.0)))))

(event `UpdateScore`
  (params (MyTeamScore :type Integer))
  (`/Engine/EditorBlueprintResources/ActorMacros.Switch Has Authority`
    (:`Remote`
      (bind _output_get (set `self.MyTeamScore` (select `bool` (`self.ButtonPushed`) :`false` MyTeamScore)))
      (bind _outactors (`GameplayStatics.GetAllActorsOfClass` "/Game/RestrictedAssets/Tutorials/Lunar/Labu/COPY_UTHUD.COPY_UTHUD_C"))
      (`/Game/RestrictedAssets/Tutorials/Lunar/Labu/COPY_UTHUD.UpdateHUD` (`KismetArrayLibrary.Array_Get` _outactors) (`KismetTextLibrary.Conv_IntToText` _output_get) (`KismetMathLibrary.Conv_ByteToInt` (`self.Team`))))))

(event `FxDeOuf`
  (params (Location :type "Vector Structure"))
  (bind _returnvalue (`self.K2_GetActorLocation`))
  (`|ExecutionSequence`
    (:`then_1`
      (`GameplayStatics.SpawnEmitterAtLocation` "/Game/RestrictedAssets/Effects/fabiom/Redeemer_Explosion.Redeemer_Explosion" _returnvalue)
      (`GameplayStatics.SpawnEmitterAtLocation` "/Game/RestrictedAssets/Weapons/Weapon_Effects/Particles/Redeemer/PFX_RedeemerBoom.PFX_RedeemerBoom" _returnvalue)
      (`GameplayStatics.SpawnEmitterAtLocation` "/Game/RestrictedAssets/Weapons/Weapon_Effects/Particles/Redeemer/PFX_Redeemer_PreBoom.PFX_Redeemer_PreBoom" _returnvalue)
      (`KismetSystemLibrary.Delay` 0.15)
      (`GameplayStatics.SpawnEmitterAtLocation` "/Game/RestrictedAssets/Weapons/Weapon_Effects/Particles/Redeemer/PFX_NewRedeemerExp.PFX_NewRedeemerExp" _returnvalue))))

(fn `UserConstructionScript`
  (bind _returnvalue (select `byte` (`self.Team`) :`0` (struct :`R` 1.0 :`G` 0.03 :`B` 0.03 :`A` 1.0) :`1` (struct :`R` 0.03 :`G` 0.03 :`B` 1.0 :`A` 1.0) :!type "LinearColor Structure"))
  (`MeshComponent.SetVectorParameterValueOnMaterials` (`self.Cylinder`) "Color" (`KismetMathLibrary.Conv_LinearColorToVector` _returnvalue))
  (`ArrowComponent.SetArrowColor_New` (`self.Sign_StartScoringDistance`) _returnvalue)
  (`SceneComponent.K2_SetRelativeLocation` (`self.Sign_StartScoringDistance`) (`KismetMathLibrary.MakeVector` (`self.StartScoringDistance`)) false false)
  (set `self.DistanceOffset` (+ (`SphereComponent.SphereRadius` (`self.Sphere`)) 40.0)))