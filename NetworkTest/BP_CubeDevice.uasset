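; BP_CubeDevice is a network-test cube gun that spawns a cube in front of the player camera when Q is pressed, polled on Tick.
; With authority, it spawns BP_DebugCube if player 0's pawn owns it.
; Remotes call CubeSpawnClient with their PlayerState, whose Authority branch spawns BP_DestructBloc, using the matching PlayerArray index as the camera manager index.
; OnStartedFiring is empty.
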(event `self.ReceiveBeginPlay`)

(event `self.OnStartedFiring`)

(event `self.ReceiveTick`
  (params (DeltaSeconds :type "Float (single-precision)"))
  (bind _returnvalue (`GameplayStatics.GetPlayerCameraManager` 0))
  (if (`PlayerController.WasInputKeyJustPressed` (`GameplayStatics.GetPlayerController` 0) "Q")
    (`KismetSystemLibrary.PrintString` "Cube gun")
    (`/Engine/EditorBlueprintResources/ActorMacros.Switch Has Authority`
      (:`Authority`
        ;[1 1 1] Server to client
        (if (== (`self.GetOwner`) (`GameplayStatics.GetPlayerPawn` 0))
          (`|SpawnActorFromClass` "/Game/RestrictedAssets/Tutorials/Lunar/NetworkTest/BP_DebugCube.BP_DebugCube_C" (`KismetMathLibrary.MakeTransform` (+ (`PlayerCameraManager.GetCameraLocation` _returnvalue) (* (`self.GetActorForwardVector` _returnvalue) 600.0))) "Undefined" "OverrideRootScale")))
      (:`Remote`
        ;[1 1 1] Client to Server
        (`self.CubeSpawnClient` (`Pawn.PlayerState` (`GameplayStatics.GetPlayerPawn` 0)))))))

(event `CubeSpawnClient`
  (params (PlayerState :type "Actor Object Reference"))
  (`/Engine/EditorBlueprintResources/ActorMacros.Switch Has Authority`
    (:`Authority`
      (for (_array_element _array_index) (`GameStateBase.PlayerArray` (`GameplayStatics.GetGameState`))
        (if (== _array_element PlayerState)
          (bind _returnvalue (`GameplayStatics.GetPlayerCameraManager` _array_index))
          (`|SpawnActorFromClass` "/Game/RestrictedAssets/Tutorials/Lunar/Corentin/DestructCube/BP_DestructBloc.BP_DestructBloc_C" (`KismetMathLibrary.MakeTransform` (+ (`PlayerCameraManager.GetCameraLocation` _returnvalue) (* (`KismetMathLibrary.GetForwardVector` (`PlayerCameraManager.GetCameraRotation` _returnvalue)) 600.0))) "Undefined" "OverrideRootScale"))))))

(fn `UserConstructionScript`)