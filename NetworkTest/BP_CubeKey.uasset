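; Network test Blueprint that polls players' Q key on the server and prints a red "player N says: Cube!" message.
; On Tick, with authority, it checks player controller indices 0 through 20 for the key press.
; Authority BeginPlay waits briefly, then loops over all PlayerControllers with an empty body.
; Disconnected leftovers include adding a cube component with an ID per controller and iterating the GameState PlayerArray.
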(event `self.ReceiveBeginPlay`
  (`/Engine/EditorBlueprintResources/ActorMacros.Switch Has Authority`
    (:`Authority`
      (`KismetSystemLibrary.Delay` 1.0)
      (bind _outactors (`GameplayStatics.GetAllActorsOfClass` "/Script/Engine.PlayerController"))
      (for (_array_element _array_index) _outactors
        _))))

(event `self.ReceiveTick`
  (params (DeltaSeconds :type "Float (single-precision)"))
  (`/Engine/EditorBlueprintResources/ActorMacros.Switch Has Authority`
    (:`Authority`
      (for _index (range 21)
        (if (`PlayerController.WasInputKeyJustPressed` (`GameplayStatics.GetPlayerController` _index) "Q")
          (`KismetSystemLibrary.PrintString` (`KismetStringLibrary.Concat_StrStr` "player " (`KismetStringLibrary.Conv_IntToString` _index) " says: Cube!") true true (struct :`R` 1.0 :`A` 1.0)))))))

(fn `UserConstructionScript`)