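; BP_CubeComponent is a component, apparently for network testing, that spawns debug cubes in front of a player's camera.
; On BeginPlay it prints its owner's name, and on Tick it polls the Q key on the player controller indexed by PCId.
; A press calls FireCube, which stores a point a fixed distance along that camera's forward vector and spawns a BP_DebugCube there.
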(event `FireCube`
  (bind _returnvalue (`GameplayStatics.GetPlayerCameraManager` (`self.PCId`)))
  (bind _returnvalue_2 (+ (`PlayerCameraManager.GetCameraLocation` _returnvalue) (* (`Actor.GetActorForwardVector` _returnvalue) 600.0) (0.0 0.0 0.0)))
  (set `self.CubeLoc` _returnvalue_2)
  (`|SpawnActorFromClass` "/Game/RestrictedAssets/Tutorials/Lunar/NetworkTest/BP_DebugCube.BP_DebugCube_C" (`KismetMathLibrary.MakeTransform` _returnvalue_2) "Undefined" "OverrideRootScale"))

(event `self.ReceiveBeginPlay`
  (`KismetSystemLibrary.PrintString` (`KismetStringLibrary.Concat_StrStr` "owner is:" (`KismetSystemLibrary.GetDisplayName` (`self.GetOwner`))) true true (struct :`G` 0.66 :`B` 1.0 :`A` 1.0) 10.0))

(event `self.ReceiveTick`
  (params (DeltaSeconds :type "Float (single-precision)"))
  (if (`PlayerController.WasInputKeyJustPressed` (`GameplayStatics.GetPlayerController` (`self.PCId`)) "Q")
    (`self.FireCube`)
    (`KismetSystemLibrary.PrintString` "CUBE")))