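; Destructible block actor that bursts into particles when fractured and removes itself when its health runs out.
; The destructible mesh's fracture event calls FX, which spawns the PS_Destruct emitter at the hit point, oriented from the reversed hit direction.
; Any damage lowers Life, and dropping below zero sets a near-zero lifespan to destroy the actor.
; BeginPlay only prints a debug message.
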(event `self.ReceiveBeginPlay`
  (`KismetSystemLibrary.PrintString` "I'm Alive" true true (struct :`G` 0.66 :`B` 1.0 :`A` 1.0) 10.0))

(event `FX`
  (params (HitPoint :type "Vector Structure") (HitDir :type "Vector Structure"))
  (`GameplayStatics.SpawnEmitterAtLocation` "/Game/RestrictedAssets/Tutorials/Lunar/Corentin/DestructCube/PS_Destruct.PS_Destruct" HitPoint (`KismetMathLibrary.FindLookAtRotation` (0.0 0.0 0.0) (* HitDir -1.0))))

(event `self.Block1_RK_DM.OnComponentFracture`
  (params (HitPoint :type "Vector Structure (by ref)") (HitDirection :type "Vector Structure (by ref)"))
  (`self.FX` HitPoint HitDirection))

(event `self.ReceiveAnyDamage`
  (params (Damage :type "Float (single-precision)") (DamageType :type "DamageType Object Reference") (InstigatedBy :type "Controller Object Reference") (DamageCauser :type "Actor Object Reference"))
  (bind _output_get (set `self.Life` (- (`self.Life`) Damage)))
  (if (< _output_get 0.0)
    (`self.SetLifeSpan` 0.01)))

(fn `UserConstructionScript`)