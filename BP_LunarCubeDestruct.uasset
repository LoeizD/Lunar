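; Destructible lunar cube actor with replicated life and scale, destroyed by point or radial damage.
; It starts without collision until SetGoodMat applies the world cube material, enables collision and clears the ScaleUpdate flag.
; Damage feeds HitCube, where the authority reduces Life unless scaling or broken, then expires the actor below zero.
; RepNotifies apply actor scale and drive the material's Hit parameter from Life.
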(event `self.ReceiveBeginPlay`
  (`PrimitiveComponent.SetCollisionEnabled` (`self.S_CubeLunar_DM`) "NoCollision"))

(event `self.ReceiveTick`
  (params (DeltaSeconds :type "Float (single-precision)")))

(event `SetGoodMat`
  (bind _s_cubelunar_dm (`self.S_CubeLunar_DM`))
  (`/Engine/EditorBlueprintResources/ActorMacros.Switch Has Authority`
    (:`Authority`
      (`KismetSystemLibrary.PrintString` "Auth"))
    (:`Remote`
      (`KismetSystemLibrary.PrintString` "Rem")))
  (`PrimitiveComponent.SetMaterial` _s_cubelunar_dm 0 "/Game/RestrictedAssets/Tutorials/Lunar/Corentin/M_WorldCube.M_WorldCube")
  (`PrimitiveComponent.SetCollisionEnabled` _s_cubelunar_dm "QueryAndPhysics")
  (set `self.ScaleUpdate` false))

(event `self.ReceiveAnyDamage`
  (params (Damage :type "Float (single-precision)") (DamageType :type "DamageType Object Reference") (InstigatedBy :type "Controller Object Reference") (DamageCauser :type "Actor Object Reference")))

(event `HitCube`
  (params (HitLoc :type "Vector Structure") (Dammage :type "Float (double-precision)"))
  (`/Engine/EditorBlueprintResources/ActorMacros.Switch Has Authority`
    (:`Authority`
      (if (`self.ScaleUpdate`)
        _
        (elif (not (`self.BreakMesh`))
          (bind _output_get (set `self.Life` (- (`self.Life`) Dammage)))
          (`|ExecutionSequence`
            (:`then_1`
              (if (< _output_get 0.0)
                (`self.SetLifeSpan` 0.01)))))))))

(event `self.ReceiveRadialDamage`
  (params (DamageReceived :type "Float (single-precision)") (DamageType :type "DamageType Object Reference") (Origin :type "Vector Structure") (HitInfo :type "HitResult Structure (by ref)") (InstigatedBy :type "Controller Object Reference") (DamageCauser :type "Actor Object Reference"))
  (`self.HitCube` Origin DamageReceived))

(event `self.ReceivePointDamage`
  (params (Damage :type "Float (single-precision)") (DamageType :type "DamageType Object Reference") (HitLocation :type "Vector Structure") (HitNormal :type "Vector Structure") (HitComponent :type "PrimitiveComponent Object Reference") (BoneName :type Name) (ShotFromDirection :type "Vector Structure") (InstigatedBy :type "Controller Object Reference") (DamageCauser :type "Actor Object Reference") (HitInfo :type "HitResult Structure (by ref)"))
  (`self.HitCube` HitLocation Damage))

(fn `OnRep_Life`
  (`MeshComponent.SetScalarParameterValueOnMaterials` (`self.S_CubeLunar_DM`) "Hit" (/ (`self.Life`) 100.0)))

(fn `OnRep_Scale`
  (`self.SetActorScale3D` (`self.Scale`)))

(fn `UserConstructionScript`)